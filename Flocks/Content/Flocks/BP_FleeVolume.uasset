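; BP_FleeVolume is a predator actor that hunts flock boids (BP_FlocksPawn) and kills those it touches.
; Each Tick it turns toward its target boid and moves at it at a fast constant speed without sweeping.
; Whenever the target is invalid, it picks a random replacement from all BP_FlocksPawn actors in the level.
; Its Sphere component's begin overlap calls Die on any flock pawn it hits, whether targeted or not.
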(event `self.ReceiveTick`
  (params (DeltaSeconds :type "Float (single-precision)"))
  (bind _returnvalue (`self.K2_GetActorLocation`))
  (bind _returnvalue_2 (`self.K2_GetActorLocation` (`self.Boid`)))
  (`self.Boid`
    (:`then`
      (`self.K2_SetActorRotation` (`KismetMathLibrary.Conv_VectorToRotator` (- _returnvalue_2 _returnvalue)))
      (`self.K2_SetActorLocation` (`KismetMathLibrary.VInterpTo_Constant` _returnvalue _returnvalue_2 DeltaSeconds 8000.0)))
    (:`else`
      (bind _outactors (`GameplayStatics.GetAllActorsOfClass` "/Game/Flocks/BP_FlocksPawn.BP_FlocksPawn_C"))
      (set `self.Boid` (`|GetArrayItem` _outactors (`KismetMathLibrary.RandomIntegerInRange` 0 (`KismetArrayLibrary.Array_Length` _outactors)))))))

(event `self.Sphere.OnComponentBeginOverlap`
  (params (OverlappedComponent :type "PrimitiveComponent Object Reference") (OtherActor :type "Actor Object Reference") (OtherComp :type "PrimitiveComponent Object Reference") (OtherBodyIndex :type Integer) (bFromSweep :type Boolean) (SweepResult :type "HitResult Structure (by ref)"))
  (bind _asbp_flocks_pawn (cast `/Game/Flocks/BP_FlocksPawn` OtherActor))
  (`/Game/Flocks/BP_FlocksPawn.Die` _asbp_flocks_pawn))

(fn `UserConstructionScript`)